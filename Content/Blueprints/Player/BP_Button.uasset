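; BP_Button is a player-folder button that activates an array of linked movable objects, then enters a cooldown.
; Activate passes through a DoOnce gate, calls Activate on each array element and swaps the button material to show cooldown.
; A Delay inside the loop leads to ResetTimer, also called by Reset, which reopens the gate and restores the material chosen by ColorGrey.
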(event `self.ReceiveBeginPlay`
  (`parent.ReceiveBeginPlay`)
  (if (`self.ColorGrey`)
    (`PrimitiveComponent.SetMaterial` (`self.Button`) 0 "/Game/Materials/M_AssetPlatform.M_AssetPlatform")))

(event `self.Activate`
  ;[1 1 1] Call activate on all the movable objects in the array
  (`/Engine/EditorBlueprintResources/StandardMacros.DoOnce` false :!label _label
    (:`Completed`
      (for _array_element (`self.Array`)
        (`self.Activate` _array_element)
        ;[1 1 1] Set material to indicate that the object is in cooldown
        (`PrimitiveComponent.SetMaterial` (`self.Button`) 0 "/Game/Materials/M_BasicAsset03.M_BasicAsset03")
        (`KismetSystemLibrary.Delay` (`self.Cooldown`))
        (`self.ResetTimer`)))))

(event `ResetTimer`
  (bind _button (`self.Button`))
  ;[1 1 1] Reset timer after cooldown and reset material to normal
  (if (`self.ColorGrey`)
    (`PrimitiveComponent.SetMaterial` _button 0 "/Game/Materials/M_AssetPlatform.M_AssetPlatform")
    (goto _label :!via `Reset`)
    (else
      (`PrimitiveComponent.SetMaterial` _button 0 "/Game/Materials/M_BasicAsset04.M_BasicAsset04")
      (goto _label :!via `Reset`))))

(event `self.Reset`
  (`self.ResetTimer`))

(fn `UserConstructionScript`
  (`parent.UserConstructionScript`))