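; Player character that picks up and uses items, activates interactables, jumps and respawns at a stored location and rotation.
; Tick pitches the camera with control rotation, box-traces ahead for the closest BP_BaseItem and clears CurrentItem once no longer attached to the player.
; AttachItem snaps that closest item to ItemSocket as CurrentItem for UseObject to trigger.
; Interact runs a similar trace, activating every BP_BaseInteractable hit.
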(event `self.ReceiveTick`
  (params (DeltaSeconds :type "Float (single-precision)"))
  (bind (_returnvalue_roll _returnvalue_pitch) (`KismetMathLibrary.BreakRotator` (`self.GetControlRotation`)))
  (bind _camera (`self.Camera`))
  (bind _returnvalue (`SceneComponent.K2_GetComponentLocation` (`self.Camera`)))
  (bind _returnvalue_2 (`SceneComponent.K2_GetComponentLocation` _camera))
  (bind _returnvalue_3 (`SceneComponent.K2_GetComponentRotation` _camera))
  (`|ExecutionSequence`
    (:`then_0`
      (`SceneComponent.K2_SetRelativeRotation` (`self.Camera`) (`KismetMathLibrary.MakeRotator` 0.0 _returnvalue_pitch) false false))
    (:`then_1`
      ;[1 1 1] Check what the closest item in range is
      (set `self.ClosestItem` null)
      (bind _outhits (`KismetSystemLibrary.BoxTraceMultiForObjects` _returnvalue_2 (+ _returnvalue_2 (* (`KismetMathLibrary.GetForwardVector` _returnvalue_3) (`self.InteractRange`))) (0.0 16.0 16.0) _returnvalue_3 (`|MakeArray` "ObjectTypeQuery7" :!type "EObjectTypeQuery Enum")))
      (for _array_element _outhits
        (bind _asbp_base_item (cast `/Game/Blueprints/Player/BP_BaseItem` (`.HitActor` (`GameplayStatics.BreakHitResult` _array_element))))
        (`/Engine/EditorBlueprintResources/StandardMacros.IsValid` (`self.ClosestItem`)
          (:`Is Valid`
            (`/Engine/EditorBlueprintResources/StandardMacros.CompareFloat` (`KismetMathLibrary.Vector_DistanceSquared` (`self.K2_GetActorLocation` _asbp_base_item) _returnvalue) (`KismetMathLibrary.Vector_DistanceSquared` _returnvalue (`self.K2_GetActorLocation` (`self.ClosestItem`)))
              (:`<`
                (set `self.ClosestItem` _asbp_base_item))))
          (:`Is Not Valid`
            (set `self.ClosestItem` _asbp_base_item)))))
    (:`then_2`
      (bind _currentitem (`self.CurrentItem`)
        (:`then`
          (if (not (== (`self.GetAttachParentActor` _currentitem) self))
            (set `self.CurrentItem` null)))
        (:`else`)))))

(event `self.ReceiveBeginPlay`
  ;[1 1 1] Jumping
  (set `self.JumpMaxHoldTime` 0.125)
  (set `self.JumpMaxCount` 1))

(event `UseObject`
  (params (IsStart :type Boolean))
  ;[1 1 1] Use object ability
  (bind _currentitem (`self.CurrentItem`)
    (:`then`
      (`/Game/Blueprints/Player/BP_BaseItem.UseItem` _currentitem))
    (:`else`)))

(event `AttachItem`
  (bind _itemsocket (`self.ItemSocket`))
  (bind _closestitem (`self.ClosestItem`))
  ;[1 1 1] Attach the weapon
  (`/Engine/EditorBlueprintResources/StandardMacros.IsValid` _closestitem
    (:`Is Valid`
      (`self.K2_SetActorTransform` _closestitem (`SceneComponent.K2_GetComponentToWorld` _itemsocket) false false)
      (`self.K2_AttachToComponent` (`self.ClosestItem`) _itemsocket "None" "SnapToTarget" "SnapToTarget" "SnapToTarget" true)
      (set `self.CurrentItem` (`self.ClosestItem`)))))

(event `Interact`
  (bind _camera (`self.Camera`))
  (bind _returnvalue (`SceneComponent.K2_GetComponentLocation` _camera))
  (bind _returnvalue_2 (`SceneComponent.K2_GetComponentRotation` _camera))
  ;[1 1 1] Activate an interactable
  (bind _outhits (`KismetSystemLibrary.BoxTraceMultiForObjects` _returnvalue (+ _returnvalue (* (`KismetMathLibrary.GetForwardVector` _returnvalue_2) (`self.InteractRange`))) (0.0 16.0 16.0) _returnvalue_2 (`|MakeArray` "ObjectTypeQuery8" :!type "EObjectTypeQuery Enum")))
  (for _array_element _outhits
    (bind _asbp_base_interactable (cast `/Game/Blueprints/Player/BP_BaseInteractable` (`.HitActor` (`GameplayStatics.BreakHitResult` _array_element))))
    (`/Game/Blueprints/Player/BP_BaseInteractable.Activate` _asbp_base_interactable)))

(event `Respawn`
  ;[1 1 1] Sets respawn point and rotation
  (`self.K2_SetActorTransform` (`self.RespawnLocation`) false true)
  (`Controller.SetControlRotation` (`self.GetController` (`GameplayStatics.GetPlayerCharacter` 0)) (`self.RespawnRotation`)))

(fn `UserConstructionScript`
  (`parent.UserConstructionScript`))