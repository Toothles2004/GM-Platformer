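; Player weapon that fires a projectile when its UseItem event runs, limited by a cooldown.
; A DoOnce gate lets the first shot fire instantly, then a timer resets it after the cooldown.
; Each shot traces from player 0's camera out to the weapon's range, then spawns the projectile at FireSocket aimed at the hit point, or along the socket's own rotation when nothing is hit.
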(event `self.UseItem`
  ;[1 1 1] Handle shoot gun action
  (if true
    (`/Engine/EditorBlueprintResources/StandardMacros.DoOnce` false :!label _label
      (:`Completed`
        ;;[1 1 1] Instant first shoot
        (`self.SpawnProjectile`)
        (`KismetSystemLibrary.K2_SetTimerDelegate` (delegate `ResetTimer`) (`self.Cooldown`))))))

(event `ResetTimer`
  ;[1 1 1] Handle shoot gun action
  (goto _label :!via `Reset`))

(event `SpawnProjectile`
  (bind _returnvalue (`SceneComponent.K2_GetComponentLocation` (`self.FireSocket`)))
  (bind (_returnvalue_location _returnvalue_rotation) (`KismetMathLibrary.BreakTransform` (`SceneComponent.K2_GetComponentToWorld` (`self.GetComponentByClass` (`GameplayStatics.GetPlayerCharacter` 0) "/Script/Engine.CameraComponent"))))
  (bind _returnvalue_2 (`KismetMathLibrary.GetForwardVector` _returnvalue_rotation))
  ;[1 1 1] Spawn the projectile
  (bind _outhit (`KismetSystemLibrary.LineTraceSingle` (+ _returnvalue_location (* _returnvalue_2 10.0)) (+ (* _returnvalue_2 (`self.Range`)) _returnvalue_location) "TraceTypeQuery1"))
  (if (`GameplayStatics.BreakHitResult` _outhit)
    ;;[1 1 1] Shoot where the player is looking
    (`|SpawnActorFromClass` (`self.PrimaryProjectileClass`) (`KismetMathLibrary.MakeTransform` _returnvalue (`KismetMathLibrary.FindLookAtRotation` _returnvalue (`.Location` (`GameplayStatics.BreakHitResult` _outhit)))) "Undefined" "MultiplyWithRoot" null null)
    (else
      ;;[1 1 1] If there is no target shoot straight
      (`|SpawnActorFromClass` (`self.PrimaryProjectileClass`) (`SceneComponent.K2_GetComponentToWorld` (`self.FireSocket`)) "Undefined" "MultiplyWithRoot" null null))))

(fn `UserConstructionScript`
  (`parent.UserConstructionScript`))