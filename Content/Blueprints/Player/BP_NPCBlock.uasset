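; BP_NPCBlock is a physics NPC block that "dies" on entering a BP_Killzone.
; On overlap it notifies BP_GameInstance of the kill and lowers its collision mass scale.
; A looping timer then repeatedly zeroes linear and angular velocity and rotates the block along the player-to-block line, intended as looking at the player.
; The block destroys itself when it leaves the killzone.
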(event `self.ReceiveActorBeginOverlap`
  (params (OtherActor :type "Actor Object Reference"))
  ;[1 1 1] Slow down when hitting killzone and look at player
  (cast `/Game/Blueprints/Player/BP_Killzone` OtherActor)
  (`|ExecutionSequence`
    (:`then_0`
      ;[1 1 1] set text and cube to dead
      (bind _asbp_game_instance (cast `/Game/Blueprints/Player/BP_GameInstance` (`GameplayStatics.GetGameInstance`)))
      (`/Game/Blueprints/Player/BP_GameInstance.NPCBlockKilled` _asbp_game_instance))
    (:`then_1`
      (`PrimitiveComponent.SetMassScale` (`self.Collision`) "None" 0.2)
      (`KismetSystemLibrary.K2_SetTimerDelegate` (delegate `SlowDown`) 0.1 true))))

(event `SlowDown`
  (bind _collision (`self.Collision`))
  (bind _collision_2 (`self.Collision`))
  ;[1 1 1] Slow down when hitting killzone and look at player
  ;;[1 1 1] Slow down velocity
  (`PrimitiveComponent.SetPhysicsLinearVelocity` _collision (0.0 0.0 0.0) false "None")
  (`PrimitiveComponent.SetPhysicsAngularVelocityInDegrees` _collision (0.0 0.0 0.0) false "None")
  (`SceneComponent.K2_SetWorldRotation` _collision_2 (`KismetMathLibrary.FindLookAtRotation` (`self.K2_GetActorLocation` (`GameplayStatics.GetPlayerPawn` 0)) (`SceneComponent.K2_GetComponentLocation` _collision_2)) false false))

(event `self.ReceiveActorEndOverlap`
  (params (OtherActor :type "Actor Object Reference"))
  ;[1 1 1] Destroy actor after leaving killzone
  (cast `/Game/Blueprints/Player/BP_Killzone` OtherActor)
  (`self.K2_DestroyActor`))

(fn `UserConstructionScript`
  (`parent.UserConstructionScript`))