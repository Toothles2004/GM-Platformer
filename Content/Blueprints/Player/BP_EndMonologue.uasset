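; End-of-game trigger that plays a narrator monologue chosen by how many of the player's companions died.
; The first player overlap, gated by DoOnce, counts the false NPCBlockAlive, NPCCylinderAlive and CubeAlive flags on BP_GameInstance.
; A switch on that death count queues one of four endings, best to worst, through NarrateText, with only the opening line interrupting current narration.
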(event `self.ReceiveActorBeginOverlap`
  (params (OtherActor :type "Actor Object Reference"))
  (cast `/Game/Blueprints/Player/BP_PlayerCharacter` OtherActor)
  (`/Engine/EditorBlueprintResources/StandardMacros.DoOnce` false
    (:`Completed`
      (bind _asbp_game_instance (cast `/Game/Blueprints/Player/BP_GameInstance` (`GameplayStatics.GetGameInstance`)))
      (if (not (`/Game/Blueprints/Player/BP_GameInstance.NPCBlockAlive` _asbp_game_instance))
        (`/Engine/EditorBlueprintResources/StandardMacros.IncrementInt` (`self.Dead`)
          (:`  `
            _)))
      (if (not (`/Game/Blueprints/Player/BP_GameInstance.NPCCylinderAlive` _asbp_game_instance))
        (`/Engine/EditorBlueprintResources/StandardMacros.IncrementInt` (`self.Dead`)
          (:`  `
            _)))
      (if (not (`/Game/Blueprints/Player/BP_GameInstance.CubeAlive` _asbp_game_instance))
        (`/Engine/EditorBlueprintResources/StandardMacros.IncrementInt` (`self.Dead`)
          (:`  `
            _)))
      (switch `int` (`self.Dead`)
        (:`0`
          (`/Game/Blueprints/Player/BP_GameInstance.NarrateText` _asbp_game_instance "Congratulations, you made it!!!" true)
          (`/Game/Blueprints/Player/BP_GameInstance.NarrateText` _asbp_game_instance "I hope you had fun, you got the best ending" false)
          (`/Game/Blueprints/Player/BP_GameInstance.NarrateText` _asbp_game_instance "You were able to get everyone to help you get to the end" false)
          (`/Game/Blueprints/Player/BP_GameInstance.NarrateText` _asbp_game_instance "You can be proud of yourself" false)
          (`/Game/Blueprints/Player/BP_GameInstance.NarrateText` _asbp_game_instance "It's time for me to go now, goodbye" false))
        (:`1`
          (`/Game/Blueprints/Player/BP_GameInstance.NarrateText` _asbp_game_instance "You made it to the end!!" true)
          (`/Game/Blueprints/Player/BP_GameInstance.NarrateText` _asbp_game_instance "Hope you had fun" false)
          (`/Game/Blueprints/Player/BP_GameInstance.NarrateText` _asbp_game_instance "This is definitely one of the better endings" false)
          (`/Game/Blueprints/Player/BP_GameInstance.NarrateText` _asbp_game_instance "You got 2 friends to help you get to the end" false)
          (`/Game/Blueprints/Player/BP_GameInstance.NarrateText` _asbp_game_instance "Maybe we'll meet again someday, but for now we'll have to say \ngoodbye" false)
          (`/Game/Blueprints/Player/BP_GameInstance.NarrateText` _asbp_game_instance "Have a nice day" false))
        (:`2`
          (`/Game/Blueprints/Player/BP_GameInstance.NarrateText` _asbp_game_instance "I guess you made it to the end" true)
          (`/Game/Blueprints/Player/BP_GameInstance.NarrateText` _asbp_game_instance "You only got 1 friend to help you" false)
          (`/Game/Blueprints/Player/BP_GameInstance.NarrateText` _asbp_game_instance "I still can't believed you actually killed them" false)
          (`/Game/Blueprints/Player/BP_GameInstance.NarrateText` _asbp_game_instance "I hope you realize that making a friend or 2 could actually benefit you " false)
          (`/Game/Blueprints/Player/BP_GameInstance.NarrateText` _asbp_game_instance "Maybe in the moment it seems easier to put people aside" false)
          (`/Game/Blueprints/Player/BP_GameInstance.NarrateText` _asbp_game_instance "But in the long run it will benefit you more to actually make friends" false)
          (`/Game/Blueprints/Player/BP_GameInstance.NarrateText` _asbp_game_instance "I guess I will go now, take care" false))
        (:`3`
          (`/Game/Blueprints/Player/BP_GameInstance.NarrateText` _asbp_game_instance "Well, here you are...." true)
          (`/Game/Blueprints/Player/BP_GameInstance.NarrateText` _asbp_game_instance "This is it, this is the end...." false)
          (`/Game/Blueprints/Player/BP_GameInstance.NarrateText` _asbp_game_instance "I hope you're happy" false)
          (`/Game/Blueprints/Player/BP_GameInstance.NarrateText` _asbp_game_instance "You killed 2 of my friends and abandoned the friend i tried giving you" false)
          (`/Game/Blueprints/Player/BP_GameInstance.NarrateText` _asbp_game_instance "I hope you realize that if you keep abandoning everyone around you,  \nyou will eventually meet difficulties you can't handle alone" false)
          (`/Game/Blueprints/Player/BP_GameInstance.NarrateText` _asbp_game_instance "This is definitely the worst ending you could have gotten" false)
          (`/Game/Blueprints/Player/BP_GameInstance.NarrateText` _asbp_game_instance "If you did this just to see what i would say then congrats, \nyou're truly evil" false)
          (`/Game/Blueprints/Player/BP_GameInstance.NarrateText` _asbp_game_instance "I will take my leave now, I could have been your friend" false)
          (`/Game/Blueprints/Player/BP_GameInstance.NarrateText` _asbp_game_instance "But now i'm not so sure...." false))))))

(fn `UserConstructionScript`)