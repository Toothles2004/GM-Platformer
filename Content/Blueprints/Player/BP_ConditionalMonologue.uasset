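; BP_ConditionalMonologue is an overlap-triggered actor that plays a one-time narration when the player character enters it, with the line depending on whether an NPC is alive.
; The NPCBlock or NPCCylinder toggle selects which alive flag to read from BP_GameInstance, with NPCBlock taking priority.
; It sends Text to NarrateText if that NPC lives or neither toggle is set, otherwise ConditionalText, without interrupting.
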(event `self.ReceiveActorBeginOverlap`
  (params (OtherActor :type "Actor Object Reference"))
  (cast `/Game/Blueprints/Player/BP_PlayerCharacter` OtherActor)
  (`/Engine/EditorBlueprintResources/StandardMacros.DoOnce` false
    (:`Completed`
      (bind _asbp_game_instance (cast `/Game/Blueprints/Player/BP_GameInstance` (`GameplayStatics.GetGameInstance`)))
      (if (`self.NPCBlock`)
        (if (`/Game/Blueprints/Player/BP_GameInstance.NPCBlockAlive` _asbp_game_instance)
          (`/Game/Blueprints/Player/BP_GameInstance.NarrateText` _asbp_game_instance (`self.Text`) false :!label _label)
          (else
            (`/Game/Blueprints/Player/BP_GameInstance.NarrateText` _asbp_game_instance (`self.ConditionalText`) false :!label _label_2)))
        (elif (`self.NPCCylinder`)
          (if (`/Game/Blueprints/Player/BP_GameInstance.NPCCylinderAlive` _asbp_game_instance)
            (goto _label)
            (else
              (goto _label_2)))
          (else
            (goto _label)))))))

(fn `UserConstructionScript`
  (`parent.UserConstructionScript`))