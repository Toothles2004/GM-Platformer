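; Item stand that swaps its held item with the player's on Activate, acting as a switch when that item is a BP_ActivationCube.
; Items are reattached between the stand's Socket and the player's ItemSocket, and each cube transfer calls Activate on every linked Array entry.
; Tick sets the body material to show cube presence and also activates the linked entries if a cube gets detached elsewhere.
; An unconnected MovableBlock MoveToOrigin branch never runs.
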(event `self.ReceiveBeginPlay`
  (`parent.ReceiveBeginPlay`))

(event `self.ReceiveTick`
  (params (DeltaSeconds :type "Float (single-precision)"))
  ;[1 1 1] Change material to indicate activity (in this case turns green when activation block is current item)
  (`parent.ReceiveTick` DeltaSeconds)
  (bind _current_item (`self.Current Item`)
    (:`then`
      (if (== (`self.GetAttachParentActor` _current_item) self)
        (cast `/Game/Blueprints/Player/BP_ActivationCube` (`self.Current Item`)
          (:`then`
            (for _ (`self.Array`)
              (`PrimitiveComponent.SetMaterial` (`self.Body`) 0 "/Game/Materials/M_BasicAsset03.M_BasicAsset03")))
          (:`CastFailed`
            (`PrimitiveComponent.SetMaterial` (`self.Body`) 0 "/Game/Materials/M_BasicAsset04.M_BasicAsset04" :!label _label)))
        (else
          (cast `/Game/Blueprints/Player/BP_ActivationCube` (`self.Current Item`))
          (for _array_element (`self.Array`)
            (`self.Activate` _array_element)
            (set `self.Current Item` null :!label _label_2)
            (goto _label)))))
    (:`else`
      (goto _label_2))))

(event `self.Activate`
  (bind _returnvalue (`GameplayStatics.GetPlayerCharacter` 0))
  (`|ExecutionSequence`
    (:`then_0`
      ;[1 1 1] Clear items from previous activate
      (set `self.StandItem` null)
      (set `self.PlayerItem` null))
    (:`then_1`
      ;[1 1 1] Get items for event
      (bind _current_item (`self.Current Item`)
        (:`then`
          (set `self.StandItem` _current_item))
        (:`else`)))
    (:`then_2`
      (bind _asbp_player_character (cast `/Game/Blueprints/Player/BP_PlayerCharacter` (`GameplayStatics.GetPlayerCharacter` 0)))
      (set `self.PlayerItem` (`/Game/Blueprints/Player/BP_PlayerCharacter.CurrentItem` _asbp_player_character)))
    (:`then_3`
      ;[1 1 1] Attach stand item to player
      (bind _standitem (`self.StandItem`)
        (:`then`
          (bind _asbp_player_character_2 (cast `/Game/Blueprints/Player/BP_PlayerCharacter` _returnvalue))
          (`self.K2_AttachToComponent` _standitem (`/Game/Blueprints/Player/BP_PlayerCharacter.ItemSocket` _asbp_player_character_2) "None" "KeepRelative" "KeepRelative" "KeepRelative" true)
          (bind _output_get (set `/Game/Blueprints/Player/BP_PlayerCharacter.CurrentItem` _standitem _asbp_player_character_2))
          (cast `/Game/Blueprints/Player/BP_ActivationCube` _output_get)
          (for _array_element (`self.Array`)
            (`self.Activate` _array_element)))
        (:`else`
          (bind _asbp_player_character_3 (cast `/Game/Blueprints/Player/BP_PlayerCharacter` _returnvalue))
          (set `/Game/Blueprints/Player/BP_PlayerCharacter.CurrentItem` null _asbp_player_character_3))))
    (:`then_4`
      ;[1 1 1] Attach player item to stand
      (bind _playeritem (`self.PlayerItem`)
        (:`then`
          (`self.K2_AttachToComponent` _playeritem (`self.Socket`) "None" "KeepRelative" "KeepRelative" "KeepRelative" true)
          (bind _output_get_2 (set `self.Current Item` _playeritem))
          (cast `/Game/Blueprints/Player/BP_ActivationCube` _output_get_2)
          (for _array_element_2 (`self.Array`)
            (`self.Activate` _array_element_2)))
        (:`else`
          (set `self.Current Item` null))))
    (:`then_5`)))

(fn `UserConstructionScript`
  (`parent.UserConstructionScript`))