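; BP_HitInteractable is a shootable switch that activates linked movable objects, such as doors, when a BP_BaseProjectile overlaps it.
; A DoOnce gate blocks repeat hits while it loops through the object array, calling Activate on each and swapping the body material to show cooldown.
; After a delay, TimerReset restores the material and reopens the gate, and the Reset event triggers the same path.
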(event `self.ReceiveActorBeginOverlap`
  (params (OtherActor :type "Actor Object Reference"))
  ;[1 1 1] If hit by bullet open door
  (cast `/Game/Blueprints/Player/BP_BaseProjectile` OtherActor)
  ;;[1 1 1] Call activate on all the movable objects in the array
  (`/Engine/EditorBlueprintResources/StandardMacros.DoOnce` false :!label _label
    (:`Completed`
      (for _array_element (`self.Array`)
        (`self.Activate` _array_element)
        ;;[1 1 1] Set material to indicate that the object is in cooldown
        (`PrimitiveComponent.SetMaterial` (`self.Body`) 0 "/Game/Materials/M_BasicAsset03.M_BasicAsset03")
        (`KismetSystemLibrary.Delay` (`self.Cooldown`))
        (`self.TimerReset`)))))

(event `TimerReset`
  ;[1 1 1] Reset timer after cooldown and reset material to normal
  (`PrimitiveComponent.SetMaterial` (`self.Body`) 0 "/Game/Materials/M_BasicAsset04.M_BasicAsset04")
  (goto _label :!via `Reset`))

(event `self.Reset`
  (`self.TimerReset`))

(fn `ResetTimer`)

(fn `UserConstructionScript`
  (`parent.UserConstructionScript`))