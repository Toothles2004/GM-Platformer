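; BP_MovableBlock is a block whose Body moves between Origin and Target component locations when activated.
; Each Activate starts a timed MoveComponentTo over TravelTime and flips MoveToOrigin, so successive calls alternate direction.
; Pause stops the move and clears ShouldMove, which gates both Activate and Reset and is never set back here.
; Reset stops any move, snaps Body to Origin and clears the direction flag.
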(event `self.ReceiveBeginPlay`
  (`parent.ReceiveBeginPlay`))

(event `self.Activate`
  ;[1 1 1] Move platform
  (if (`self.Should move`)
    (`|ExecutionSequence`
      (:`then_0`
        (`KismetSystemLibrary.MoveComponentTo` (`self.Body`) (`SceneComponent.RelativeLocation` (select `bool` (`self.MoveToOrigin`) :`false` (`self.Target`) :`true` (`self.Origin`))) (struct) false false (`self.TravelTime`) :!label _label))
      (:`then_1`
        (set `self.MoveToOrigin` (not (`self.MoveToOrigin`)))))))

(event `self.Pause`
  ;[1 1 1] Move platform
  (set `self.Should move` false)
  (goto _label :!via `Stop`))

(event `self.Reset`
  ;[1 1 1] Go back to start location on reset
  (if (`self.Should move`)
    (`|ExecutionSequence`
      (:`then_0`
        (goto _label :!via `Stop`))
      (:`then_1`
        (`KismetSystemLibrary.MoveComponentTo` (`self.Body`) (`SceneComponent.RelativeLocation` (`self.Origin`)) (struct) false false 0.0)
        (set `self.MoveToOrigin` false)))))

(fn `UserConstructionScript`
  (`parent.UserConstructionScript`))