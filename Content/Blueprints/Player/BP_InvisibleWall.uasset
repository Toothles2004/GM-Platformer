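; BP_InvisibleWall is a toggleable blocking wall actor in the Player folder.
; Its Activate event flips an Active flag, then sets the Collision component to QueryAndPhysics when active or NoCollision when inactive.
; BeginPlay, overlap and Tick are disabled stubs, and the construction script only calls its parent, so this graph changes collision only through Activate.
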(event `self.Activate`
  (bind _output_get (set `self.Active` (not (`self.Active`))))
  (if _output_get
    (`PrimitiveComponent.SetCollisionEnabled` (`self.Collision`) "QueryAndPhysics")
    (else
      (`PrimitiveComponent.SetCollisionEnabled` (`self.Collision`) "NoCollision"))))

(fn `UserConstructionScript`
  (`parent.UserConstructionScript`))