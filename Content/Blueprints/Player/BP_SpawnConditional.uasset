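; BP_SpawnConditional is a spawner that creates the activation cube, NPCs and a weapon based on alive flags stored in BP_GameInstance.
; On BeginPlay it checks each flag and spawns the matching actor at one of its marker components.
; The two NPCs take only the marker's location, with hardcoded rotation and scale.
; The weapon shares the cylinder NPC's flag, so it spawns only alongside that NPC.
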(event `self.ReceiveBeginPlay`
  (bind _returnvalue_location (`KismetMathLibrary.BreakTransform` (`SceneComponent.K2_GetComponentToWorld` (`self.Block`))))
  (bind _returnvalue_location_2 (`KismetMathLibrary.BreakTransform` (`SceneComponent.K2_GetComponentToWorld` (`self.Cylinder`))))
  (bind _asbp_game_instance (cast `/Game/Blueprints/Player/BP_GameInstance` (`GameplayStatics.GetGameInstance`)))
  (`|ExecutionSequence`
    (:`then_0`
      (if (`/Game/Blueprints/Player/BP_GameInstance.CubeAlive` _asbp_game_instance)
        (`|SpawnActorFromClass` "/Game/Blueprints/Player/BP_ActivationCube.BP_ActivationCube_C" (`SceneComponent.K2_GetComponentToWorld` (`self.ActivationBlock`)) "Undefined" "MultiplyWithRoot" null null)))
    (:`then_1`
      (if (`/Game/Blueprints/Player/BP_GameInstance.NPCBlockAlive` _asbp_game_instance)
        (`|SpawnActorFromClass` "/Game/Blueprints/Player/BP_NPCBlock.BP_NPCBlock_C" (`KismetMathLibrary.MakeTransform` _returnvalue_location (struct :`Yaw` 90.0) (2.5 2.0 2.0)) "Undefined" "MultiplyWithRoot" null null)))
    (:`then_2`
      (if (`/Game/Blueprints/Player/BP_GameInstance.NPCCylinderAlive` _asbp_game_instance)
        (`|SpawnActorFromClass` "/Game/Blueprints/Player/BP_NPCCylinder.BP_NPCCylinder_C" (`KismetMathLibrary.MakeTransform` _returnvalue_location_2 (struct :`Yaw` -90.0) (2.6 2.6 2.6)) "Undefined" "MultiplyWithRoot" null null)
        (`|SpawnActorFromClass` "/Game/Blueprints/Player/BP_Weapon01.BP_Weapon01_C" (`SceneComponent.K2_GetComponentToWorld` (`self.Gun`)) "Undefined" "MultiplyWithRoot" null null)))))

(fn `UserConstructionScript`)