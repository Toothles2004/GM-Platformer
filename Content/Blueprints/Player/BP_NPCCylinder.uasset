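; BP_NPCCylinder is an NPC actor that gets killed when a BP_BaseProjectile overlaps it.
; On that overlap it tilts its collision component to start a fall and notifies BP_GameInstance through NPCCylinderKilled.
; After a short delay it calls Pause on each entry in its array of interactables to stop them moving.
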(event `self.ReceiveActorBeginOverlap`
  (params (OtherActor :type "Actor Object Reference"))
  ;[1 1 1] Engage movement so character falls
  (cast `/Game/Blueprints/Player/BP_BaseProjectile` OtherActor)
  (`SceneComponent.K2_SetWorldRotation` (`self.Collsision`) (struct :`Pitch` -5.0 :`Roll` -5.0) false false)
  ;[1 1 1] Tell the game instance that the character was killed
  (bind _asbp_game_instance (cast `/Game/Blueprints/Player/BP_GameInstance` (`GameplayStatics.GetGameInstance`)))
  (`/Game/Blueprints/Player/BP_GameInstance.NPCCylinderKilled` _asbp_game_instance)
  ;[1 1 1] Stop interactables from moving
  (`KismetSystemLibrary.Delay` 0.5)
  (for _array_element (`self.Array`)
    (`self.Pause` _array_element)))

(fn `UserConstructionScript`
  (`parent.UserConstructionScript`))