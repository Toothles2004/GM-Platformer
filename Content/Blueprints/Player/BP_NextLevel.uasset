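; BP_NextLevel is a level transition trigger that opens the level named by LevelName when an actor overlaps it.
; When the player character overlaps, it checks the linked ItemStand for a BP_ActivationCube and, if found, calls ActivationCubeAlive on BP_GameInstance before the level change.
; The level opens whatever the result of those checks, including for non-player overlaps.
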(event `self.ReceiveBeginPlay`
  (`parent.ReceiveBeginPlay`))

(event `self.ReceiveActorBeginOverlap`
  (params (OtherActor :type "Actor Object Reference"))
  (cast `/Game/Blueprints/Player/BP_PlayerCharacter` OtherActor
    (:`then`
      (bind _current_item (`/Game/Blueprints/Player/BP_ItemStand.Current Item` (`self.ItemStand`))
        (:`then`
          (cast `/Game/Blueprints/Player/BP_ActivationCube` _current_item
            (:`then`
              (bind _asbp_game_instance (cast `/Game/Blueprints/Player/BP_GameInstance` (`GameplayStatics.GetGameInstance`))
                (:`then`
                  (`/Game/Blueprints/Player/BP_GameInstance.ActivationCubeAlive` _asbp_game_instance))
                (:`CastFailed`
                  _)))
            (:`CastFailed`
              _)))
        (:`else`
          _)))
    (:`CastFailed`
      _))
  (`GameplayStatics.OpenLevel` (`self.LevelName`)))

(fn `UserConstructionScript`
  (`parent.UserConstructionScript`))